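; Stamping machine Blueprint that reshapes a printed part when StartStamping is called.
; It copies the incoming mesh to PrintedPartToStamp, then immediately swaps the part's own cone, cube or cylinder mesh for a matching stamped shape.
; A timeline then moves the stamp head along Z.
; CanPlayAnim blocks replaying the animation until it finishes, but does not block the mesh swap.
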(event `StartStamping`
  (params (CurrentPrintedPartToStamp :type "/Game/MyLogic/Phase_1/Printed_Part/BP/BP_Printed_Part Object Reference"))
  (bind _staticmesh (`StaticMeshComponent.StaticMesh` (`/Game/MyLogic/Phase_1/Printed_Part/BP/BP_Printed_Part.SM_Printed_Part` CurrentPrintedPartToStamp)))
  (set `self.Current Printed Part to Stamp` CurrentPrintedPartToStamp)
  (set `self.PrintedPartStaticMeshRefIn` _staticmesh)
  (`StaticMeshComponent.SetStaticMesh` (`self.PrintedPartToStamp`) _staticmesh)
  (`|ExecutionSequence`
    (:`then_0`
      (if (== (`self.PrintedPartStaticMeshRefIn`) "/Game/StarterContent/Shapes/Shape_Cone.Shape_Cone")
        (`StaticMeshComponent.SetStaticMesh` (`/Game/MyLogic/Phase_1/Printed_Part/BP/BP_Printed_Part.SM_Printed_Part` (`self.Current Printed Part to Stamp`)) "/Game/StarterContent/Shapes/Shape_NarrowCapsule.Shape_NarrowCapsule")
        (elif (== (`self.PrintedPartStaticMeshRefIn`) "/Game/StarterContent/Shapes/Shape_Cube.Shape_Cube")
          (`StaticMeshComponent.SetStaticMesh` (`/Game/MyLogic/Phase_1/Printed_Part/BP/BP_Printed_Part.SM_Printed_Part` (`self.Current Printed Part to Stamp`)) "/Game/StarterContent/Shapes/Shape_Pipe.Shape_Pipe")
          (elif (== (`self.PrintedPartStaticMeshRefIn`) "/Game/StarterContent/Shapes/Shape_Cylinder.Shape_Cylinder")
            (`StaticMeshComponent.SetStaticMesh` (`/Game/MyLogic/Phase_1/Printed_Part/BP/BP_Printed_Part.SM_Printed_Part` (`self.Current Printed Part to Stamp`)) "/Game/StarterContent/Shapes/Shape_Plane.Shape_Plane")))))
    (:`then_1`
      (if (`self.CanPlayAnim?`)
        (set `self.CanPlayAnim?` false)
        (bind (_direction _stampheadz) (`Timeline|StampingAnimGraph` :!via `PlayFromStart`)
          (:`Update`
            (`SceneComponent.K2_SetRelativeLocation` (`self.SM_StampingMachineHaead`) (`KismetMathLibrary.MakeVector` 0.0 0.0 _stampheadz) false false))
          (:`Finished`
            (set `self.CanPlayAnim?` true)))))))

(fn `UserConstructionScript`)