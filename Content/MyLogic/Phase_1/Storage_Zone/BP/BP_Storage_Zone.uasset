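; BP_Storage_Zone is a storage area that spawns BP_Printed_Part actors to display printed parts and links.
; On BeginPlay it caches the world locations of two start markers as running spawn cursors.
; PlacePrintedParts spawns a part with the supplied static mesh and steps its cursor along Y, forming a row.
; PlaceLinks spawns parts with a fixed trim mesh and steps its cursor along Z, forming a vertical stack.
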(event `self.ReceiveBeginPlay`
  (bind _output_get (set `self.PartSpawnLocation` (`SceneComponent.K2_GetComponentLocation` (`self.PartSpawnStart`))))
  (set `self.CurrentPrintedPartSpawnLocation` _output_get)
  (bind _output_get_2 (set `self.LinkSpawnLocation` (`SceneComponent.K2_GetComponentLocation` (`self.LinkSpawnStart`))))
  (set `self.CurrentLinkSpawnLocation` _output_get_2))

(event `PlacePrintedParts`
  (params (PrintedPartRefIn :type "StaticMesh Object Reference"))
  (bind _returnvalue (`|SpawnActorFromClass` "/Game/MyLogic/Phase_1/Printed_Part/BP/BP_Printed_Part.BP_Printed_Part_C" (`KismetMathLibrary.MakeTransform` (`self.CurrentPrintedPartSpawnLocation`)) "Undefined" "OverrideRootScale" null null))
  (`StaticMeshComponent.SetStaticMesh` (`/Game/MyLogic/Phase_1/Printed_Part/BP/BP_Printed_Part.SM_Printed_Part` _returnvalue) PrintedPartRefIn)
  (set `self.CurrentPrintedPartSpawnLocation` (`KismetMathLibrary.MakeVector` (.x (`self.CurrentPrintedPartSpawnLocation`)) (+ (.y (`self.CurrentPrintedPartSpawnLocation`)) (`self.PrintedPartSpacerX`)) (.z (`self.CurrentPrintedPartSpawnLocation`)))))

(event `PlaceLinks`
  (bind _returnvalue (`|SpawnActorFromClass` "/Game/MyLogic/Phase_1/Printed_Part/BP/BP_Printed_Part.BP_Printed_Part_C" (`KismetMathLibrary.MakeTransform` (`self.CurrentLinkSpawnLocation`)) "Undefined" "OverrideRootScale" null null))
  (`StaticMeshComponent.SetStaticMesh` (`/Game/MyLogic/Phase_1/Printed_Part/BP/BP_Printed_Part.SM_Printed_Part` _returnvalue) "/Game/StarterContent/Shapes/Shape_Trim_90_Out.Shape_Trim_90_Out")
  (set `self.CurrentLinkSpawnLocation` (`KismetMathLibrary.MakeVector` (.x (`self.CurrentLinkSpawnLocation`)) (.y (`self.CurrentLinkSpawnLocation`)) (+ (.z (`self.CurrentLinkSpawnLocation`)) (`self.LinkSpacerZ`)))))

(fn `UserConstructionScript`)