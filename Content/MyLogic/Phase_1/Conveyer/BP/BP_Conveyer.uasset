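; BP_Conveyer is a conveyor station that routes printed parts to the stamping machine and storage zone through two overlap triggers.
; TriggerBox stores the entering part and starts stamping on it, unless its mesh is Connection.
; TableTransportationTrigger destroys the part and has the storage zone place links for Connection meshes or printed parts for others.
; BeginPlay caches the movement spline's two world endpoints, which this graph does not otherwise use.
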(event `self.ReceiveBeginPlay`
  (bind _printedpart_movementtrajectory (`self.PrintedPart_MovementTrajectory`))
  (set `self.MovementTrajectory_Start` (`SplineComponent.GetLocationAtSplinePoint` _printedpart_movementtrajectory 0 "World"))
  (set `self.MovementTrajectory_End` (`SplineComponent.GetLocationAtSplinePoint` _printedpart_movementtrajectory 1 "World")))

(event `self.TableTransportationTrigger.OnComponentBeginOverlap`
  (params (OverlappedComponent :type "PrimitiveComponent Object Reference") (OtherActor :type "Actor Object Reference") (OtherComp :type "PrimitiveComponent Object Reference") (OtherBodyIndex :type Integer) (bFromSweep :type Boolean) (SweepResult :type "HitResult Structure (by ref)"))
  (bind _asbp_printed_part (cast `/Game/MyLogic/Phase_1/Printed_Part/BP/BP_Printed_Part` OtherActor))
  (set `self.PrintedPartMeshRef` (`StaticMeshComponent.StaticMesh` (`/Game/MyLogic/Phase_1/Printed_Part/BP/BP_Printed_Part.SM_Printed_Part` _asbp_printed_part)))
  (`self.K2_DestroyActor` _asbp_printed_part)
  (if (== (`self.PrintedPartMeshRef`) "/Game/Blender/Printed_Parts/Connection.Connection")
    (bind _returnvalue (`GameplayStatics.GetActorOfClass` "/Game/MyLogic/Phase_1/Storage_Zone/BP/BP_Storage_Zone.BP_Storage_Zone_C"))
    (`/Game/MyLogic/Phase_1/Storage_Zone/BP/BP_Storage_Zone.PlaceLinks` _returnvalue)
    (else
      (bind _returnvalue_2 (`GameplayStatics.GetActorOfClass` "/Game/MyLogic/Phase_1/Storage_Zone/BP/BP_Storage_Zone.BP_Storage_Zone_C"))
      (`/Game/MyLogic/Phase_1/Storage_Zone/BP/BP_Storage_Zone.PlacePrintedParts` _returnvalue_2 (`self.PrintedPartMeshRef`)))))

(event `self.TriggerBox.OnComponentBeginOverlap`
  (params (OverlappedComponent :type "PrimitiveComponent Object Reference") (OtherActor :type "Actor Object Reference") (OtherComp :type "PrimitiveComponent Object Reference") (OtherBodyIndex :type Integer) (bFromSweep :type Boolean) (SweepResult :type "HitResult Structure (by ref)"))
  (bind _asbp_printed_part (cast `/Game/MyLogic/Phase_1/Printed_Part/BP/BP_Printed_Part` OtherActor))
  (set `self.As BP Printed Part` _asbp_printed_part)
  (if (not (== (`StaticMeshComponent.StaticMesh` (`/Game/MyLogic/Phase_1/Printed_Part/BP/BP_Printed_Part.SM_Printed_Part` _asbp_printed_part)) "/Game/Blender/Printed_Parts/Connection.Connection"))
    (bind _returnvalue (`GameplayStatics.GetActorOfClass` "/Game/MyLogic/Phase_1/Stamping_Machine/BP/BP_Stamping_machine.BP_Stamping_machine_C"))
    (`/Game/MyLogic/Phase_1/Stamping_Machine/BP/BP_Stamping_machine.StartStamping` _returnvalue (`self.As BP Printed Part`))))

(fn `UserConstructionScript`)