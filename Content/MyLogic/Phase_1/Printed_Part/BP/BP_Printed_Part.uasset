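; BP_Printed_Part is a printed part actor that travels along the conveyor.
; On BeginPlay it finds the BP_Conveyer in the level and caches its trajectory start and end points.
; The StartTransportation event plays a timeline that lerps the actor's location between those two points, without sweep.
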(event `self.ReceiveBeginPlay`
  (bind _returnvalue (`GameplayStatics.GetActorOfClass` "/Game/MyLogic/Phase_1/Conveyer/BP/BP_Conveyer.BP_Conveyer_C"))
  (set `self.Movement Trajectory End In` (`/Game/MyLogic/Phase_1/Conveyer/BP/BP_Conveyer.MovementTrajectory_End` _returnvalue))
  (set `self.Movement Trajectory Start In` (`/Game/MyLogic/Phase_1/Conveyer/BP/BP_Conveyer.MovementTrajectory_Start` _returnvalue)))

(event `Start Transportation`
  (params (CurrentPrintedPart :type "/Game/MyLogic/Phase_1/Printed_Part/BP/BP_Printed_Part Object Reference"))
  (bind (_direction _transport_alpha) (`Timeline|PrintedPartMovementGraph`)
    (:`Update`
      (`self.K2_SetActorLocation` (`KismetMathLibrary.VLerp` (`self.Movement Trajectory Start In`) (`self.Movement Trajectory End In`) _transport_alpha)))))

(fn `UserConstructionScript`)