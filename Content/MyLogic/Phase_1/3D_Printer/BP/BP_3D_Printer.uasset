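; 3D printer actor for Phase 1 that, once the player first enters its trigger, prints a sequence of parts onto the conveyor.
; Each cycle plays the printer animation, spawns a BP_Printed_Part at the conveyor's trajectory end point, starts its transport and sets its mesh.
; A self-retriggering DoN with a delay repeats each part type by its configured count, then resets and advances through the parallel mesh and count arrays.
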(event `self.ReceiveBeginPlay`
  (bind _returnvalue (`GameplayStatics.GetActorOfClass` "/Game/MyLogic/Phase_1/Conveyer/BP/BP_Conveyer.BP_Conveyer_C"))
  (set `self.Movement Trajectory End In` (`/Game/MyLogic/Phase_1/Conveyer/BP/BP_Conveyer.MovementTrajectory_End` _returnvalue)))

(event `self.Phase1_Trigger.OnComponentBeginOverlap`
  (params (OverlappedComponent :type "PrimitiveComponent Object Reference") (OtherActor :type "Actor Object Reference") (OtherComp :type "PrimitiveComponent Object Reference") (OtherBodyIndex :type Integer) (bFromSweep :type Boolean) (SweepResult :type "HitResult Structure (by ref)"))
  (cast `/Game/FirstPersonBP/Blueprints/FirstPersonCharacter` OtherActor)
  (`/Engine/EditorBlueprintResources/StandardMacros.DoOnce` false
    (:`Completed`
      (set `self.NumberOfCurrentPrintedPartType` (`|GetArrayItem` (`self.NumberOf_PrintedParts`) (`self.Index`)) :!label _label)
      (bind _counter (`/Engine/EditorBlueprintResources/StandardMacros.Do N` (`self.NumberOfCurrentPrintedPartType`) :!label _label_2)
        (:`Exit`
          (`SkeletalMeshComponent.PlayAnimation` (`self.SK_3D_Printer`) null false)
          (bind _returnvalue (`|SpawnActorFromClass` "/Game/MyLogic/Phase_1/Printed_Part/BP/BP_Printed_Part.BP_Printed_Part_C" (`KismetMathLibrary.MakeTransform` (`self.Movement Trajectory End In`)) "Undefined" "OverrideRootScale" null null))
          (`/Game/MyLogic/Phase_1/Printed_Part/BP/BP_Printed_Part.Start Transportation` _returnvalue null)
          (`StaticMeshComponent.SetStaticMesh` (`/Game/MyLogic/Phase_1/Printed_Part/BP/BP_Printed_Part.SM_Printed_Part` _returnvalue) (`|GetArrayItem` (`self.PrintedPart_Types`) (`self.Index`)))
          (`KismetSystemLibrary.Delay` 5.0)
          (if (== (`self.NumberOfCurrentPrintedPartType`) _counter)
            (`/Engine/EditorBlueprintResources/StandardMacros.IncrementInt` (`self.Index`)
              (:`  `
                (`self.ResetCounter`)
                (goto _label)))
            (else
              (goto _label_2))))))))

(event `ResetCounter`
  (goto _label_2 :!via `Reset`))

(fn `UserConstructionScript`)