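; BP_3DPrinter simulates a 3D printer that feeds randomly chosen printed parts onto a conveyor in Phase 1.
; On BeginPlay it enables player input and takes its spawn point from the BP_Conveyer's transport start location.
; The StartPhase1 input runs a DoN and Delay loop that spawns BP_PrintedPart actors at intervals, up to NumberOfPrintedParts.
; Each part gets a random mesh from PrintedPartTypes and immediately starts transportation.
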(event `self.ReceiveBeginPlay`
  (`self.EnableInput` (`GameplayStatics.GetPlayerController` 0))
  (bind _returnvalue (`GameplayStatics.GetActorOfClass` "/Game/MyLogic/Phase1/Blueprints/BP_Conveyer.BP_Conveyer_C"))
  (set `self.Spawn Transform Location` (`/Game/MyLogic/Phase1/Blueprints/BP_Conveyer.Transport Start Location` _returnvalue)))

(event `InputAction|StartPhase1`
  (params (Key :type "Key Structure"))
  (:`Pressed`
    (`/Engine/EditorBlueprintResources/StandardMacros.Do N` (`self.NumberOfPrintedParts`) :!label _label
      (:`Exit`
        (bind _returnvalue (`|SpawnActorFromClass` "/Game/MyLogic/Phase1/Blueprints/BP_PrintedPart.BP_PrintedPart_C" (`KismetMathLibrary.MakeTransform` (`self.Spawn Transform Location`)) "Undefined" "OverrideRootScale" null null))
        (`StaticMeshComponent.SetStaticMesh` (`/Game/MyLogic/Phase1/Blueprints/BP_PrintedPart.PrintedPart_PH` _returnvalue) (`|GetArrayItem` (`self.PrintedPartTypes`) (`KismetMathLibrary.RandomIntegerInRange` 0 3)))
        (`/Game/MyLogic/Phase1/Blueprints/BP_PrintedPart.StartTransportation` _returnvalue)
        (`KismetSystemLibrary.Delay` (`self.Duration`))
        (goto _label)))))

(fn `UserConstructionScript`)