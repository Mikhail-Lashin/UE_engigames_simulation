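; BP_PrintedPart is an actor for a printed part that moves along a conveyor.
; On BeginPlay it finds the BP_Conveyer in the level and copies its transport start and end locations.
; StartTransportation plays the TransportationGraph timeline, whose alpha track lerps the part's location from start to end without sweeping.
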(event `self.ReceiveBeginPlay`
  (bind _returnvalue (`GameplayStatics.GetActorOfClass` "/Game/MyLogic/Phase1/Blueprints/BP_Conveyer.BP_Conveyer_C"))
  (set `self.Transport Start Location In` (`/Game/MyLogic/Phase1/Blueprints/BP_Conveyer.Transport Start Location` _returnvalue))
  (set `self.Transport End Location In` (`/Game/MyLogic/Phase1/Blueprints/BP_Conveyer.Transport End Location` _returnvalue)))

(event `StartTransportation`
  (bind (_direction _alpha_transportation_key) (`Timeline|TransportationGraph`)
    (:`Update`
      (`self.K2_SetActorLocation` (`KismetMathLibrary.VLerp` (`self.Transport Start Location In`) (`self.Transport End Location In`) _alpha_transportation_key)))))

(fn `UserConstructionScript`)