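; BP_Conveyer is a conveyor actor that reacts to BP_PrintedPart actors entering its trigger box.
; On BeginPlay it caches the world locations of the first two spline points as transport start and end, though no movement logic uses them here.
; On overlap it swaps the part's PrintedPartPH mesh to Shape_Sphere unless that mesh is Shape_Trim_90_Out.
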(event `self.ReceiveBeginPlay`
  (bind _spline (`self.Spline`))
  (set `self.Transport Start Location` (`SplineComponent.GetLocationAtSplinePoint` _spline 0 "World"))
  (set `self.Transport End Location` (`SplineComponent.GetLocationAtSplinePoint` _spline 1 "World")))

(event `self.TriggerBox.OnComponentBeginOverlap`
  (params (OverlappedComponent :type "PrimitiveComponent Object Reference") (OtherActor :type "Actor Object Reference") (OtherComp :type "PrimitiveComponent Object Reference") (OtherBodyIndex :type Integer) (bFromSweep :type Boolean) (SweepResult :type "HitResult Structure (by ref)"))
  (bind _asbp_printed_part (cast `/Game/MyLogic/Phase1/Blueprints/BP_PrintedPart` OtherActor))
  (if (not (== (`StaticMeshComponent.StaticMesh` (`/Game/MyLogic/Phase1/Blueprints/BP_PrintedPart.PrintedPart_PH` _asbp_printed_part)) "/Game/StarterContent/Shapes/Shape_Trim_90_Out.Shape_Trim_90_Out"))
    (`StaticMeshComponent.SetStaticMesh` (`/Game/MyLogic/Phase1/Blueprints/BP_PrintedPart.PrintedPart_PH` _asbp_printed_part) "/Game/StarterContent/Shapes/Shape_Sphere.Shape_Sphere")))

(fn `UserConstructionScript`)